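; BP_Hitbox is a melee-style hitbox actor that applies effects to living actors on other teams when they overlap it.
; On BeginPlay it adds overlap spheres snapped to the AttachTo sockets on the instigator's skeletal mesh, or a single sphere on itself if none are given.
; Overlaps are filtered by IGetHit, team and liveness, and HitActors limits each target to one hit.
; Hits send EffectsToApply, a hit-connect gameplay event to PlayerPawn, and a success message to the instigator.
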(event `self.ReceiveBeginPlay`
  (bind _attachto (`self.AttachTo`))
  (if (> (`KismetArrayLibrary.Array_Length` _attachto) 0)
    (for _array_element _attachto
      (bind _returnvalue (`AddComponent|NODE_AddSphereComponent-3` :`bManualAttachment` true))
      (`PrimitiveComponent.SetCollisionResponseToChannel` _returnvalue "ECC_Pawn" "ECR_Ignore")
      (`PrimitiveComponent.SetCollisionResponseToChannel` _returnvalue "ECC_Destructible" "ECR_Overlap")
      (`SphereComponent.SetSphereRadius` _returnvalue 45.0 true)
      (`SceneComponent.K2_AttachToComponent` _returnvalue (`self.GetComponentByClass` (`self.GetInstigator`) "/Script/Engine.SkeletalMeshComponent") _array_element "SnapToTarget" "KeepRelative" "KeepRelative" true))
    (else
      (bind _returnvalue_2 (`AddComponent|NODE_AddSphereComponent-4`))
      (`PrimitiveComponent.SetCollisionResponseToChannel` _returnvalue_2 "ECC_Pawn" "ECR_Ignore")
      (`PrimitiveComponent.SetCollisionResponseToChannel` _returnvalue_2 "ECC_Destructible" "ECR_Overlap")
      (`SphereComponent.SetSphereRadius` _returnvalue_2 45.0 true))))

(event `self.ReceiveActorBeginOverlap`
  (params (OtherActor :type "Actor Object Reference"))
  (bind _returnvalue (`self.GetInstigator`))
  (bind _playerpawn (`self.PlayerPawn`))
  (if (and (`KismetSystemLibrary.IsValid` OtherActor) (!= OtherActor _playerpawn) (`KismetSystemLibrary.DoesImplementInterface` OtherActor "/Script/MyBuilder.IGetHit") (`self.IsTargetTypeValid` OtherActor))
    (bind _returnvalue_2 (message `IGetHit.IsAlive` OtherActor))
    (if _returnvalue_2
      (if (not (`KismetArrayLibrary.Array_Contains` (`self.HitActors`) OtherActor))
        (`KismetArrayLibrary.Array_Add` (`self.HitActors`) OtherActor)
        (message `IGetHit.OnGetHitByEffects` OtherActor (`self.EffectsToApply`))
        (`AbilitySystemBlueprintLibrary.SendGameplayEventToActor` _playerpawn (struct :`TagName` "notify.hit.connect"))
        (`/Engine/EditorBlueprintResources/StandardMacros.IsValid` _returnvalue
          (:`Is Valid`
            (message `HasHitbox.OnHitSuccess` _returnvalue)))))))

(fn `IsTargetTypeValid`
  (params (OtherActor :type "Actor Object Reference"))
  (returns (`Is It?` :type Boolean))
  (bind _returnvalue (message `IGetHit.GetTeam` OtherActor))
  (bind _returnvalue_2 (message `IGetHit.GetTeam` (`self.PlayerPawn`)))
  (return (!= _returnvalue_2 _returnvalue)))

(fn `UserConstructionScript`)