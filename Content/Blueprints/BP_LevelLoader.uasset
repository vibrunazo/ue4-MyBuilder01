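; BP_LevelLoader builds a randomized row of rooms at runtime from streaming levels.
; On BeginPlay it blocking-loads the Room03 level, then calls SpawnNewRoom in a short fixed loop.
; Each call creates a uniquely named streaming level instance of Room02 or Room03 at random, offsets it along Y by the iteration count, and sets it loaded and visible.
; Room01Name is unused.
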(event `SpawnNewRoom`
  (`/Engine/EditorBlueprintResources/StandardMacros.IncrementInt` (`self.Iteration`)
    (:`  `
      (bind _returnvalue (`LevelStreaming.CreateInstance` (`GameplayStatics.GetStreamingLevel` (select `int` (`KismetMathLibrary.RandomIntegerInRange` 0 1) :`0` (`self.Room02Name`) :`1` (`self.Room03Name`))) (`KismetStringLibrary.Concat_StrStr` "room" (`KismetStringLibrary.Conv_IntToString` (`self.Iteration`)))))
      (set `LevelStreaming.LevelTransform` (`KismetMathLibrary.MakeTransform` (`KismetMathLibrary.MakeVector` 0.0 (* (`self.Iteration`) 2000.0))) _returnvalue)
      (set `LevelStreaming.bShouldBeVisible` true _returnvalue)
      (set `LevelStreaming.bShouldBeLoaded` true _returnvalue))))

(event `self.ReceiveBeginPlay`
  (`GameplayStatics.LoadStreamLevel` (`self.Room03Name`) true true)
  (for _ (range 4)
    (`self.SpawnNewRoom`)))

(fn `UserConstructionScript`)