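; BP_PlayerController is a player controller that relays health, death and win events to the game's HUD.
; It caches a BP_HUD reference on BeginPlay, forwards health updates to it, and triggers its game-over handling when the player dies.
; On a win it calls the parent handler, unpossesses the pawn, notifies the HUD, immediately opens the next level by name, and restores game-only input with a hidden cursor.
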(event `self.ReceiveBeginPlay`
  (bind _asbp_hud (cast `/Game/UI/BP_HUD` (`self.GetHUD`)))
  (set `self.HUD Ref` _asbp_hud))

(event `self.OnPlayerDead`
  (`parent.OnPlayerDead`)
  (`/Game/UI/BP_HUD.OnGameOver` (`self.HUD Ref`)))

(event `self.OnWin`
  (params (NextLevel :type Name))
  (`parent.OnWin` NextLevel)
  (`self.UnPossess`)
  (`/Game/UI/BP_HUD.OnWinLevel` (`self.HUD Ref`) NextLevel)
  (`GameplayStatics.OpenLevel` NextLevel)
  (`WidgetBlueprintLibrary.SetInputMode_GameOnly` self)
  (set `self.bShowMouseCursor` false))

(fn `Update HUD Health`
  (params (NewHealth :type "Float (double-precision)"))
  (`/Game/UI/BP_HUD.Update Health` (`self.HUD Ref`) NewHealth))

(fn `UserConstructionScript`)