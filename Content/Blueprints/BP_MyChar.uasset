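; BP_MyChar is a Gameplay Ability System combat character for players and AI, with team set by controller type.
; Skill inputs drive abilities, while incoming effect specs update a widget healthbar and notify states can apply effects.
; Damage triggers a montage, camera shake and aggro blackboard write, hit pause slows CustomTimeDilation, and death launches a ragdoll.
; Falling ignores Pawn collision until a non-falling capsule hit restores it and activates GA_CancelFlyAttacks.
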(event `Key|Five`
  (params (Key :type "Key Structure"))
  (bind _abilitysystem (`self.AbilitySystem`))
  (:`Pressed`
    (`KismetSystemLibrary.PrintString` (`KismetStringLibrary.Conv_IntToString` (`AbilitySystemComponent.GetGameplayEffectCount` _abilitysystem "/Game/Abilities/GE_HitStun.GE_HitStun_C" _abilitysystem true)))))

(event `Key|Four`
  (params (Key :type "Key Structure"))
  (bind _abilitysystem (`self.AbilitySystem`))
  (:`Pressed`
    (`AbilitySystemComponent.RemoveActiveGameplayEffectBySourceEffect` _abilitysystem "/Game/Abilities/GE_HitStun.GE_HitStun_C" _abilitysystem 1)))

(event `Key|Three`
  (params (Key :type "Key Structure"))
  (:`Pressed`
    (`self.Crouch`))
  (:`Released`
    (`self.UnCrouch`)))

(event `InputAction|Skill2`
  (params (Key :type "Key Structure"))
  (bind _output_abilityclass (break `AbilityStruct` (`|GetArrayItem` (`self.Abilities`) 2)))
  (:`Pressed`
    (`AbilitySystemComponent.TryActivateAbilityByClass` (`self.AbilitySystem`) _output_abilityclass true)))

(event `InputAction|Skill1`
  (params (Key :type "Key Structure"))
  (:`Pressed`
    (`self.SetAbilityKeyDown` 0 true))
  (:`Released`
    (`self.SetAbilityKeyDown` 0)))

(event `self.ReceiveBeginPlay`
  (set `self.SkelMeshRef` (`self.Mesh`))
  (`AbilitySystemComponent.BP_ApplyGameplayEffectToSelf` :`self` (`self.AbilitySystem`) :`GameplayEffectClass` "/Game/Abilities/GE_GainControl.GE_GainControl_C")
  (`self.UpdateHealthbar`)
  (`self.GiveAbility` "/Game/Abilities/GA_CancelFlyAttacks.GA_CancelFlyAttacks_C")
  (cast `PlayerController` (`self.GetController`)
    (:`then`
      (set `self.Team` 1))
    (:`CastFailed`
      (set `self.Team` 0))))

(event `self.OnGetHitByEffects`
  (params (NewEffects :type "Array of GameplayEffectSpecHandle Structure (by ref)"))
  (for _array_element NewEffects
    (`IGetHit.OnGetHitByEffect` _array_element)))

(event `self.OnGetHitByEffect`
  (params (NewEffect :type "GameplayEffectSpecHandle Structure"))
  (`AbilitySystemComponent.BP_ApplyGameplayEffectSpecToSelf` (`self.AbilitySystem`) NewEffect)
  (`self.UpdateHealthbar`))

(event `self.OnDie`
  (bind _mesh (`self.Mesh`))
  (`KismetSystemLibrary.Delay` 0.1)
  (`parent.OnDie`)
  (`PrimitiveComponent.SetSimulatePhysics` _mesh true)
  (`PrimitiveComponent.SetCollisionEnabled` _mesh "PhysicsOnly")
  (`PrimitiveComponent.AddForce` _mesh (-50000.0 0.0 100000.0) "None" true)
  (`PrimitiveComponent.SetCollisionResponseToChannel` (`self.CapsuleComponent`) "ECC_Pawn" "ECR_Ignore")
  (`KismetSystemLibrary.Delay` 5.0)
  (`self.K2_DestroyActor`))

(event `self.OnHitPause`
  (params (Duration :type "Float (single-precision)"))
  (set `self.CustomTimeDilation` 0.01)
  (`KismetSystemLibrary.Delay` Duration)
  (set `self.CustomTimeDilation` 1.0))

(event `self.PawnSensing.OnSeePawn`
  (params (Pawn :type "Pawn Object Reference"))
  (bind _returnvalue (`AIBlueprintHelperLibrary.GetBlackboard` null))
  (bind _playerkeyname (`self.PlayerKeyName`))
  (`/Engine/EditorBlueprintResources/StandardMacros.IsValid` (`BlackboardComponent.GetValueAsObject` _returnvalue _playerkeyname)
    (:`Is Not Valid`
      (`/Engine/EditorBlueprintResources/StandardMacros.IsValid` (`BlackboardComponent.GetValueAsObject` _returnvalue (`self.LastAggroKey`))
        (:`Is Not Valid`
          (`BlackboardComponent.SetValueAsObject` _returnvalue _playerkeyname Pawn))))))

(event `self.OnJumped`)

(event `self.K2_OnMovementModeChanged`
  (params (PrevMovementMode :type "EMovementMode Enum" :default "MOVE_None") (NewMovementMode :type "EMovementMode Enum" :default "MOVE_None") (PrevCustomMode :type Byte) (NewCustomMode :type Byte))
  (if (`|EnumEquality` NewMovementMode "MOVE_Falling")
    (`PrimitiveComponent.SetCollisionResponseToChannel` (`self.CapsuleComponent`) "ECC_Pawn" "ECR_Ignore")))

(event `self.OnDamaged`
  (params (InstigatorActor :type "Actor Object Reference"))
  (bind _returnvalue (`AIBlueprintHelperLibrary.GetBlackboard` null))
  (`parent.OnDamaged` InstigatorActor)
  (`self.PlayAnimMontage` "/Game/Anims/React_Front_Small_Montage.React_Front_Small_Montage")
  (`GameplayStatics.PlayWorldCameraShake` "/Game/FX/CamShake/Shake_Hit1.Shake_Hit1_C" (`self.K2_GetActorLocation`) 0.0 1000.0)
  (`/Engine/EditorBlueprintResources/StandardMacros.IsValid` _returnvalue
    (:`Is Valid`
      (`BlackboardComponent.SetValueAsObject` _returnvalue (`self.LastAggroKey`) InstigatorActor))))

(event `self.CapsuleComponent.OnComponentHit`
  (params (HitComponent :type "PrimitiveComponent Object Reference") (OtherActor :type "Actor Object Reference") (OtherComp :type "PrimitiveComponent Object Reference") (NormalImpulse :type "Vector Structure") (Hit :type "HitResult Structure (by ref)"))
  (if (not (`NavMovementComponent.IsFalling` (`self.CharacterMovement`)))
    (`AbilitySystemComponent.TryActivateAbilityByClass` (`self.AbilitySystem`) "/Game/Abilities/GA_CancelFlyAttacks.GA_CancelFlyAttacks_C" true)
    (`PrimitiveComponent.SetCollisionResponseToChannel` (`self.CapsuleComponent`) "ECC_Pawn" "ECR_Block")))

(event `self.CastProjectile`
  (params (ProjectileClass :type "Actor Class Reference") (NewEffects :type "Array of GameplayEffectSpecHandle Structure (by ref)"))
  (`|SpawnActorFromClass` "/Game/Blueprints/BP_Projectile.BP_Projectile_C" (`SceneComponent.K2_GetComponentToWorld` (`self.ProjSpawn`)) "Undefined" "OverrideRootScale" self NewEffects self self))

(fn `ApplyEffectFromNotify`
  (params (EffectClass :type "GameplayEffect Class Reference") (`ANS Reference` :type "/Game/Blueprints/Notifies/ANS_Base Object Reference"))
  (bind _returnvalue (`AbilitySystemComponent.BP_ApplyGameplayEffectToSelf` :`self` (`self.AbilitySystem`) :`GameplayEffectClass` EffectClass))
  (set `/Game/Blueprints/Notifies/ANS_Base.MyEffect` _returnvalue `ANS Reference`))

(fn `GetTeam`
  (returns (ReturnValue :type Integer))
  (return (`self.Team`)))

(fn `UpdateHealthbar`
  (bind _aswbp_healthbar (cast `/Game/UI/WBP_Healthbar` (`WidgetComponent.GetUserWidgetObject` (`self.Widget`))))
  (`/Game/UI/WBP_Healthbar.SetHealthText` _aswbp_healthbar (`.ReturnValue` (`AbilitySystemBlueprintLibrary.GetFloatAttributeFromAbilitySystemComponent` (`self.AbilitySystem`) (struct :`AttributeName` "Health" :`Attribute` "StructProperty'\"/Script/MyBuilder.MyAttributeSet:Health\"'" :`AttributeOwner` "Class'\"/Script/MyBuilder.MyAttributeSet\"'")))))

(fn `UserConstructionScript`)