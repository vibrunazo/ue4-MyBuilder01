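; BP_Projectile is a projectile actor that delegates hit handling to an attached BP_Hitbox.
; On BeginPlay it spawns the hitbox with the effects to apply, the owning player pawn and itself as instigator, then snaps it to itself.
; OnHitSuccess flags the hit and destroys both actors.
; BeginPlay rechecks that flag after attaching, removing the hitbox if a hit has already registered.
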(event `self.ReceiveBeginPlay`
  (bind _playerpawn (`self.PlayerPawn`))
  (bind _returnvalue (`|SpawnActorFromClass` "/Game/Blueprints/BP_Hitbox.BP_Hitbox_C" (`self.GetTransform`) "AlwaysSpawn" "OverrideRootScale" _playerpawn (`self.EffectsToApply`) (`self.AttachTo`) _playerpawn self))
  (`self.K2_AttachToActor` _returnvalue self "None" "SnapToTarget" "KeepRelative" "KeepRelative" true)
  (set `self.HitboxRef` _returnvalue)
  (if (`self.HaveHit`)
    (`self.K2_DestroyActor` _returnvalue)))

(event `self.OnHitSuccess`
  (bind _hitboxref (`self.HitboxRef`))
  (set `self.HaveHit` true)
  (`|ExecutionSequence`
    (:`then_0`
      (`/Engine/EditorBlueprintResources/StandardMacros.IsValid` _hitboxref
        (:`Is Valid`
          (`self.K2_DestroyActor` _hitboxref))))
    (:`then_1`
      (`self.K2_DestroyActor`))))

(fn `UserConstructionScript`)