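; Behavior tree decorator that decides whether the AI should chase the player.
; It passes when the blackboard player actor is valid and is either the last aggro target or no valid last aggro target exists.
; Both actors are read from blackboard keys, so a different valid aggro target blocks the chase.
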(fn `PerformConditionCheck`
  (params (OwnerActor :type "Actor Object Reference"))
  (returns (ReturnValue :type Boolean))
  (bind _returnvalue (`BTFunctionLibrary.GetBlackboardValueAsActor` (`self.LastAggro`)))
  (bind _returnvalue_2 (`BTFunctionLibrary.GetBlackboardValueAsActor` (`self.PlayerKey`)))
  (return (and (`KismetSystemLibrary.IsValid` _returnvalue_2) (or (== _returnvalue_2 _returnvalue) (not (`KismetSystemLibrary.IsValid` _returnvalue))))))