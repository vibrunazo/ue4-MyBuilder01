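; Behavior tree task that makes an AI-controlled BP_MyChar attack through the Gameplay Ability System.
; On execute, it adds movement input toward the actor stored in the player blackboard key, then tries to activate abilities matching TagToActivate.
; It finishes successfully right away without waiting for the ability or checking activation, and fails only when the pawn is not a BP_MyChar.
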(event `self.ReceiveExecuteAI`
  (params (OwnerController :type "AIController Object Reference") (ControlledPawn :type "Pawn Object Reference"))
  (bind _asbp_my_char (cast `/Game/Blueprints/BP_MyChar` ControlledPawn)
    (:`then`
      (`Pawn.AddMovementInput` _asbp_my_char (- (`Actor.K2_GetActorLocation` (`BTFunctionLibrary.GetBlackboardValueAsActor` (`self.PlayerKeyName`))) (`Actor.K2_GetActorLocation` _asbp_my_char)) 9000.0 false)
      (`AbilitySystemComponent.TryActivateAbilitiesByTag` (`MyBuilderCharacter.AbilitySystem` _asbp_my_char) (`self.TagToActivate`) true)
      (`self.FinishExecute` true))
    (:`CastFailed`
      (`self.FinishExecute` false))))