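; Anim notify state that keeps a hit-stun gameplay effect on a BP_MyChar for the length of its animation window.
; On begin, it passes GE_HitStun and itself to the character's ApplyEffectFromNotify.
; On end, it removes one stack of that effect by class, with the character's own ability system as instigator.
; Alternative removals by handle or tag, and debug prints, remain unconnected.
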(fn `Received_NotifyBegin`
  (params (MeshComp :type "SkeletalMeshComponent Object Reference") (Animation :type "AnimSequenceBase Object Reference") (TotalDuration :type "Float (double-precision)"))
  (returns (ReturnValue :type Boolean))
  (bind _asbp_my_char (cast `/Game/Blueprints/BP_MyChar` (`ActorComponent.GetOwner` MeshComp)))
  (`/Game/Blueprints/BP_MyChar.ApplyEffectFromNotify` _asbp_my_char "/Game/Abilities/GE_HitStun.GE_HitStun_C" self)
  (return false))

(fn `Received_NotifyEnd`
  (params (MeshComp :type "SkeletalMeshComponent Object Reference") (Animation :type "AnimSequenceBase Object Reference"))
  (returns (ReturnValue :type Boolean))
  (bind _asbp_my_char (cast `/Game/Blueprints/BP_MyChar` (`ActorComponent.GetOwner` MeshComp)))
  (bind _abilitysystem (`MyBuilderCharacter.AbilitySystem` _asbp_my_char))
  (`AbilitySystemComponent.RemoveActiveGameplayEffectBySourceEffect` _abilitysystem "/Game/Abilities/GE_HitStun.GE_HitStun_C" _abilitysystem 1)
  (return false))