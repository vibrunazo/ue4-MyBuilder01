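; Base trigger actor that tracks a list of characters to kill and can send the player to the next level.
; On BeginPlay it binds to the death event of each BP_MyChar in ActorList, removes each as it dies, then calls Activate once the list empties.
; Activate is empty here.
; While IsActive is set, a player-controlled pawn entering the Box calls OnWin on BP_PlayerController with NextLevel.
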(event `Activate`)

(event `OnTargetDied`
  (params (DestroyedActor :type "Actor Object Reference"))
  (`KismetArrayLibrary.Array_RemoveItem` (`self.ActorList`) DestroyedActor)
  (if (== (`KismetArrayLibrary.Array_Length` (`self.ActorList`)) 0)
    (`self.Activate`)))

(event `self.ReceiveBeginPlay`
  (for _array_element (`self.ActorList`)
    (bind _asbp_my_char (cast `/Game/Blueprints/BP_MyChar` _array_element))
    (add `MyBuilderCharacter.OnDied` _asbp_my_char (delegate `OnTargetDied`))))

(event `self.Box.OnComponentBeginOverlap`
  (params (OverlappedComponent :type "PrimitiveComponent Object Reference") (OtherActor :type "Actor Object Reference") (OtherComp :type "PrimitiveComponent Object Reference") (OtherBodyIndex :type Integer) (bFromSweep :type Boolean) (SweepResult :type "HitResult Structure (by ref)"))
  (if (`self.IsActive`)
    (bind _aspawn (cast `Pawn` OtherActor))
    (bind _asbp_player_controller (cast `/Game/Blueprints/BP_PlayerController` (`Pawn.GetController` _aspawn)))
    (`MyPlayerController.OnWin` _asbp_player_controller (`self.NextLevel`))))

(fn `UserConstructionScript`)