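; Base melee attack Gameplay Ability that plays a combo montage chosen by the current combo index.
; Montage gameplay events spawn and destroy a BP_Hitbox attached to the character mesh, passing it payload bone names and SetByCaller damage and hitstun effects.
; A connecting hit triggers hit pause and advances the combo once per activation, resetting after a timeout.
; CanCombo, set when a connected hit's active window ends, allows reactivation despite the Attacking tag.
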(event `SetComboTimer`
  (`self.AllowComboInc`)
  (if (> (- (`GameplayStatics.GetTimeSeconds`) (`self.lastCombo`)) 1.0)
    (`self.ResetCombo`)))

(event `ResetCombo`
  (set `self.CurCombo` 0))

(event `IncCombo`
  (`/Engine/EditorBlueprintResources/StandardMacros.DoOnce` false :!label _label
    (:`Completed`
      (if (< (+ (`self.CurCombo`) 1) (`KismetArrayLibrary.Array_Length` (`self.MontagesToPlays`)))
        (set `self.CurCombo` (+ (`self.CurCombo`) 1))
        (else
          (`self.ResetCombo`)))
      (set `self.lastCombo` (`GameplayStatics.GetTimeSeconds`)))))

(event `AllowComboInc`
  (goto _label :!via `Reset`))

(event `self.K2_OnEndAbility`
  (params (bWasCancelled :type Boolean))
  (`parent.K2_OnEndAbility` bWasCancelled)
  (`self.KillHitBox`))

(event `OnHitConnect`
  (message `IGetHit.OnHitPause` (`self.GetAvatarActorFromActorInfo`) (`self.Hit Pause Duration`))
  (set `self.HitConnected` true)
  (`self.IncCombo`))

(event `SpawnHitBox`
  (params (Payload :type "GameplayEventData Structure"))
  (`self.KillHitBox`)
  (bind _asbp_my_char (cast `/Game/Blueprints/BP_MyChar` (`self.GetOwningActorFromActorInfo`)))
  (bind (_asynctaskproxy _spawnedactor) (`AbilityTask_SpawnActor.SpawnActor` (struct) "/Game/Blueprints/BP_Hitbox.BP_Hitbox_C" (`self.GetEffectsToApply`) (`self.GetBonesList` Payload) _asbp_my_char _asbp_my_char)
    (:`Success`
      (`Actor.K2_AttachToComponent` _spawnedactor (`/Game/Blueprints/BP_MyChar.SkelMeshRef` _asbp_my_char) "None" "SnapToTarget" "KeepRelative" "KeepRelative" true))))

(event `OnHitActiveEnd`
  (set `self.CanCombo` (select `bool` (`self.HitConnected`) :`true` true))
  (`self.KillHitBox`))

(event `KillHitBox`
  (`/Engine/EditorBlueprintResources/StandardMacros.IsValid` (stale `SpawnHitBox` _spawnedactor)
    (:`Is Valid`
      (`Actor.K2_DestroyActor` (stale `SpawnHitBox` _spawnedactor)))))

(event `self.K2_ActivateAbility`
  (`self.K2_CommitAbility`)
  (set `self.CanCombo` false)
  (set `self.HitConnected` false)
  (`self.SetComboTimer`)
  (`AbilityTask_PlayMontageAndWait.CreatePlayMontageAndWaitProxy` "None" (`|GetArrayItem` (`self.MontagesToPlays`) (`self.CurCombo`))
    (:`then`
      (bind (_asynctaskproxy _payload) (`AbilityTask_WaitGameplayEvent.WaitGameplayEvent` (struct :`TagName` "notify.hit.start") null false false)
        (:`then`
          (`AbilityTask_WaitGameplayEvent.WaitGameplayEvent` (struct :`TagName` "notify.hit.end") null
            (:`then`
              (`AbilityTask_WaitGameplayEvent.WaitGameplayEvent` (struct :`TagName` "notify.hit.connect") null
                (:`EventReceived`
                  (`self.OnHitConnect`))))
            (:`EventReceived`
              (`self.OnHitActiveEnd`))))
        (:`EventReceived`
          (`self.SpawnHitBox` _payload))))
    (:`OnCompleted`
      (`self.KillHitBox` :!label _label_2)
      (`self.K2_EndAbility`))
    (:`OnBlendOut`
      (goto _label_2))
    (:`OnInterrupted`
      (goto _label_2))
    (:`OnCancelled`
      (goto _label_2))))

(fn `GetBonesList`
  (params (Payload :type "GameplayEventData Structure"))
  (returns (BoneName :type "Array of Name"))
  (bind _ashitbox_settings (cast `HitboxSettings` Payload_OptionalObject))
  (return (`HitboxSettings.BoneNames` _ashitbox_settings)))

(fn `GetEffectsToApply`
  (returns (EffectsToApply :type "Array of GameplayEffectSpecHandle Structure"))
  (bind _effectstoapply (`self.EffectsToApply`))
  (bind _returnvalue (`AbilitySystemBlueprintLibrary.AssignTagSetByCallerMagnitude` (`self.MakeOutgoingGameplayEffectSpec` (`self.EffectToApply`)) (struct :`TagName` "data.damage") (* -1 (`self.damage`))))
  (bind _returnvalue_2 (`AbilitySystemBlueprintLibrary.AssignTagSetByCallerMagnitude` (`self.MakeOutgoingGameplayEffectSpec` "/Game/Abilities/GE_HitStunWithDuration.GE_HitStunWithDuration_C") (struct :`TagName` "data.hitstun") (`self.HitStunDuration`)))
  (`KismetArrayLibrary.Array_Set` _effectstoapply 0 _returnvalue true)
  (`KismetArrayLibrary.Array_Set` _effectstoapply 1 _returnvalue_2 true)
  (return _effectstoapply))

(fn `K2_CanActivateAbility`
  (params (ActorInfo :type "GameplayAbilityActorInfo Structure"))
  (returns (RelevantTags :type "GameplayTagContainer Structure") (ReturnValue :type Boolean))
  (bind _returnvalue (message `GameplayTagAssetInterface.HasMatchingGameplayTag` (`.AbilitySystemComponent` (break `GameplayAbilityActorInfo` ActorInfo)) (struct :`TagName` "attacking")))
  (return (struct) (or (not _returnvalue) (`self.CanCombo`))))