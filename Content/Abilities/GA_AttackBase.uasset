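; Base gameplay ability for melee attacks that chain through an array of combo montages.
; Gameplay events during the montage spawn a hitbox carrying an effect spec on the tagged hand, then destroy it.
; A connect event triggers hit pause, advances the combo and permits reactivation despite the Attacking tag.
; The combo wraps after the last montage or resets when activation comes too long after the last hit.
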(event `SetComboTimer`
  (if (> (- (`GameplayStatics.GetTimeSeconds`) (`self.lastCombo`)) 0.5)
    (`self.ResetCombo`)))

(event `ResetCombo`
  (set `self.CurCombo` 0))

(event `IncCombo`
  (if (< (+ (`self.CurCombo`) 1) (`KismetArrayLibrary.Array_Length` (`self.MontagesToPlays`)))
    (set `self.CurCombo` (+ (`self.CurCombo`) 1))
    (else
      (`self.ResetCombo`)))
  (set `self.lastCombo` (`GameplayStatics.GetTimeSeconds`)))

(event `self.K2_OnEndAbility`
  (params (bWasCancelled :type Boolean))
  (`parent.K2_OnEndAbility` bWasCancelled)
  (`self.KillHitBox`))

(event `OnHitConnect`
  (message `IGetHit.OnHitPause` (`self.GetAvatarActorFromActorInfo`) 0.18)
  (set `self.CanCombo` true)
  (`self.IncCombo`))

(event `SpawnHitBox`
  (params (Payload :type "GameplayEventData Structure"))
  (bind _asbp_my_char (cast `/Game/Blueprints/BP_MyChar` (`self.GetOwningActorFromActorInfo`)))
  (bind (_asynctaskproxy _spawnedactor) (`AbilityTask_SpawnActor.SpawnActor` (struct) "/Game/Blueprints/BP_Hitbox.BP_Hitbox_C" (`self.MakeOutgoingGameplayEffectSpec` (`self.EffectToApply`)) _asbp_my_char)
    (:`Success`
      (`Actor.K2_AttachToComponent` _spawnedactor (`/Game/Blueprints/BP_MyChar.SkelMeshRef` _asbp_my_char) (`self.GetBoneName` Payload) "SnapToTarget" "KeepRelative" "KeepRelative" true))))

(event `KillHitBox`
  (`/Engine/EditorBlueprintResources/StandardMacros.IsValid` (stale `SpawnHitBox` _spawnedactor)
    (:`Is Valid`
      (`Actor.K2_DestroyActor` (stale `SpawnHitBox` _spawnedactor)))))

(event `self.K2_ActivateAbility`
  (`self.K2_CommitAbility`)
  (set `self.CanCombo` false)
  (`self.SetComboTimer`)
  (`AbilityTask_PlayMontageAndWait.CreatePlayMontageAndWaitProxy` "None" (`|GetArrayItem` (`self.MontagesToPlays`) (`self.CurCombo`))
    (:`then`
      (bind (_asynctaskproxy _payload) (`AbilityTask_WaitGameplayEvent.WaitGameplayEvent` (struct :`TagName` "notify.hit.start") null true false)
        (:`then`
          (`AbilityTask_WaitGameplayEvent.WaitGameplayEvent` (struct :`TagName` "notify.hit.end") null true
            (:`then`
              (`AbilityTask_WaitGameplayEvent.WaitGameplayEvent` (struct :`TagName` "notify.hit.connect") null
                (:`EventReceived`
                  (`self.OnHitConnect`))))
            (:`EventReceived`
              (`self.KillHitBox`))))
        (:`EventReceived`
          (`self.SpawnHitBox` _payload))))
    (:`OnCompleted`
      (`self.KillHitBox` :!label _label)
      (`self.K2_EndAbility`))
    (:`OnBlendOut`
      (goto _label))
    (:`OnInterrupted`
      (goto _label))
    (:`OnCancelled`
      (goto _label))))

(fn `GetBoneName`
  (params (Payload :type "GameplayEventData Structure"))
  (returns (BoneName :type Name))
  (`|SwitchGameplayTag` (`.EventTag` (break `GameplayEventData` Payload))
    (:`Default`
      _)
    (:`notify.hit.start.handr`
      _)
    (:`notify.hit.start.handl`
      (return "hand_l")))
  (return "hand_r"))

(fn `K2_CanActivateAbility`
  (params (ActorInfo :type "GameplayAbilityActorInfo Structure"))
  (returns (RelevantTags :type "GameplayTagContainer Structure") (ReturnValue :type Boolean))
  (bind _returnvalue (message `GameplayTagAssetInterface.HasMatchingGameplayTag` (`.AbilitySystemComponent` (break `GameplayAbilityActorInfo` ActorInfo)) (struct :`TagName` "attacking")))
  (return (struct) (or (not _returnvalue) (`self.CanCombo`))))