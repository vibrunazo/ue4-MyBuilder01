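; GA_BaseCast is a gameplay ability that casts a projectile from its avatar actor.
; On activation it runs the parent logic, then waits for the Notify.projectile.spawn gameplay event.
; When the event arrives, it sends CastProjectileMessage to the avatar with BP_Projectile and the effects to apply, leaving the spawn to the avatar.
; An older direct SpawnActor chain is disconnected and never runs.
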(event `OnProjectileSpawn`
  (message `CastProjectile.CastProjectile` (`self.GetAvatarActorFromActorInfo`) "/Game/Blueprints/BP_Projectile.BP_Projectile_C" (`self.GetEffectsToApply`)))

(event `self.K2_ActivateAbility`
  (`parent.K2_ActivateAbility`)
  (`AbilityTask_WaitGameplayEvent.WaitGameplayEvent` (struct :`TagName` "notify.projectile.spawn") null
    (:`EventReceived`
      (`self.OnProjectileSpawn`))))